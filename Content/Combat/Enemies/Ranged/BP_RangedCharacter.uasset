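; Ranged enemy character Blueprint that sets up its overhead UI and visual reactions to being hit or marked.
; BeginPlay creates a dynamic mesh material and fills widget components for the health bar, head display and a separate marked display.
; Hittable component events show or clear the "Marked" label.
; On hit, a timeline drives the material's FlashingAlpha parameter while SplatterComponent spawns ambrosia splatters.
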(event OnHit(Hittable)
  (params (Data :type Hittable%20Hit%20Data%20Structure))
  (Utilities|FlowControl|Sequence
    (:then_0
      (bind _alpha (Timeline|Timeline PlayFromStart)
        (:Update
          (Rendering|Material|SetScalarParameterValue (Variables|Default|GetDynMat) "FlashingAlpha" _alpha :!class /Script/Engine.MaterialInstanceDynamic))))
    (:then_1
      (Default|SpawnAmbrosiaSplatters (Variables|Default|GetSplatter_Component) 1 2))))

(event Custom|OnMarkedEnd
  (Class|HeadDisplayWidgetComponent|DeactivateDisplay (Variables|Default|GetMarkedHeadDisplay)))

(event Custom|OnMarked
  (Class|HeadDisplayWidgetComponent|IndefiniteDisplay (Variables|Default|GetMarkedHeadDisplay) "Marked"))

(event EventBeginPlay
  (bind _headdisplaywidget (Variables|Default|GetHeadDisplayWidget))
  (bind _markedheaddisplay (Variables|Default|GetMarkedHeadDisplay))
  (bind _hittable (Variables|Default|GetHittable))
  (bind _returnvalue (Rendering|Material|CreateDynamicMaterialInstance (Variables|Character|GetMesh) 0 (Rendering|Material|GetMaterial (Variables|Character|GetMesh) 0) "None" :!class /Script/Engine.PrimitiveComponent))
  (bind _output_get (Variables|Default|SetDynMat _returnvalue))
  (Rendering|Material|SetMaterial (Variables|Character|GetMesh) 0 _output_get)
  (bind _returnvalue_2 (Game|ConstructObjectfromClass "/Game/Combat/WBP_EntityHealthBar.WBP_EntityHealthBar_C" (Variables|Default|GetHealth)))
  (UserInterface|SetWidget (Variables|Default|GetHealthBar) _returnvalue_2)
  (bind _returnvalue_3 (Game|ConstructObjectfromClass "/Game/Combat/WBP_HeadDisplayWidget.WBP_HeadDisplayWidget_C" _headdisplaywidget))
  (UserInterface|SetWidget _headdisplaywidget _returnvalue_3)
  (EventDispatchers|BindEventtoOnMarked _hittable (delegate Custom|OnMarked))
  (EventDispatchers|BindEventtoOnMarkConsumed _hittable (delegate Custom|OnMarkedEnd))
  (bind _returnvalue_4 (Game|ConstructObjectfromClass "/Game/Combat/WBP_HeadDisplayWidget.WBP_HeadDisplayWidget_C" _markedheaddisplay))
  (UserInterface|SetWidget _markedheaddisplay _returnvalue_4))

(fn ConstructionScript)