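; Fast melee enemy character that presents combat feedback through overhead widgets, hit effects and an attack telegraph.
; BeginPlay builds a dynamic mesh material, health bar and head displays, including a "Marked" display toggled by Hittable mark events.
; Hits flash the material via a timeline and spawn ambrosia splatters.
; MeleeAttacker windup reveals a fill indicator whose timeline is rate-scaled to the first attack's WindupTime, then recovery or cancellation hides it.
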(event OnHit(Hittable)
  (params (Data :type Hittable%20Hit%20Data%20Structure))
  (Utilities|FlowControl|Sequence
    (:then_0
      (bind _alpha (Timeline|Timeline PlayFromStart)
        (:Update
          (Rendering|Material|SetScalarParameterValue (Variables|Default|GetDynMat) "FlashingAlpha" _alpha :!class /Script/Engine.MaterialInstanceDynamic))))
    (:then_1
      (Default|SpawnAmbrosiaSplatters (Variables|Default|GetSplatter_Component) 1 2))))

(event OnMeleeAttackCancelled(MeleeAttacker)
  (Utilities|FlowControl|Sequence
    (:then_0
      (Development|SetHiddeninGame (Variables|Default|GetParent) true true)
      (Transformation|SetRelativeScale3D (Variables|Default|GetFillParent) "1.000000,1.000000,1.000000")
      (Transformation|SetRelativeScale3D (Variables|Default|GetParent) "1.000000,1.000000,1.000000"))
    (:then_1
      (bind _scale (Timeline|IndicatorTimeline Stop)
        (:Update
          (Transformation|SetRelativeScale3D (Variables|Default|GetFillParent) (Math|Vector|MakeVector _scale 1.0 1.0)))))))

(event OnAttackStateChanged(MeleeAttacker)
  (params (NewState :type EAttackState%20Enum :default "None"))
  (if (Utilities|Enum|Equal(Enum) NewState "Windup")
    (Components|Timeline|SetPlayRate (Variables|Default|GetIndicatorTimeline) (/ 1.0 (.winduptime (Utilities|Array|Get(acopy) (Variables|/Script/LuhorPrototype.MeleeAttackChain|GetAttacks (Variables|/Script/LuhorPrototype.MeleeAttackerComponent|GetMeleeAttackChain (Variables|Default|GetMeleeAttacker)))))))
    (Development|SetHiddeninGame (Variables|Default|GetParent) false true)
    (bind _scale (Timeline|IndicatorTimeline PlayFromStart)
      (:Update
        (Transformation|SetRelativeScale3D (Variables|Default|GetFillParent) (Math|Vector|MakeVector _scale 1.0 1.0))))
    (elif (not (Utilities|Enum|Equal(Enum) NewState "Contact"))
      (if (Utilities|Enum|Equal(Enum) NewState "Recovery")
        (Development|SetHiddeninGame (Variables|Default|GetParent) true true)
        (Transformation|SetRelativeScale3D (Variables|Default|GetFillParent) "1.000000,1.000000,1.000000")
        (Transformation|SetRelativeScale3D (Variables|Default|GetParent) "1.000000,1.000000,1.000000")))))

(event Custom|OnMarkedEnd
  (Class|HeadDisplayWidgetComponent|DeactivateDisplay (Variables|Default|GetMarkedHeadDisplay)))

(event Custom|OnMarked
  (Class|HeadDisplayWidgetComponent|IndefiniteDisplay (Variables|Default|GetMarkedHeadDisplay) "Marked"))

(event EventBeginPlay
  (bind _headdisplaywidget (Variables|Default|GetHeadDisplayWidget))
  (bind _markedheaddisplay (Variables|Default|GetMarkedHeadDisplay))
  (bind _hittable (Variables|Default|GetHittable))
  (bind _returnvalue (Rendering|Material|CreateDynamicMaterialInstance (Variables|Character|GetMesh) 0 (Rendering|Material|GetMaterial (Variables|Character|GetMesh) 0) "None" :!class /Script/Engine.PrimitiveComponent))
  (bind _output_get (Variables|Default|SetDynMat _returnvalue))
  (Rendering|Material|SetMaterial (Variables|Character|GetMesh) 0 _output_get)
  (bind _returnvalue_2 (Game|ConstructObjectfromClass "/Game/Combat/WBP_EntityHealthBar.WBP_EntityHealthBar_C" (Variables|Default|GetHealth) (Variables|Default|GetStagger) (Variables|Default|GetHittable)))
  (UserInterface|SetWidget (Variables|Default|GetHealthBar) _returnvalue_2)
  (bind _returnvalue_3 (Game|ConstructObjectfromClass "/Game/Combat/WBP_HeadDisplayWidget.WBP_HeadDisplayWidget_C" _headdisplaywidget))
  (UserInterface|SetWidget _headdisplaywidget _returnvalue_3)
  (EventDispatchers|BindEventtoOnMarked _hittable (delegate Custom|OnMarked))
  (EventDispatchers|BindEventtoOnMarkConsumed _hittable (delegate Custom|OnMarkedEnd))
  (bind _returnvalue_4 (Game|ConstructObjectfromClass "/Game/Combat/WBP_HeadDisplayWidget.WBP_HeadDisplayWidget_C" _markedheaddisplay))
  (UserInterface|SetWidget _markedheaddisplay _returnvalue_4)
  (Development|SetHiddeninGame (Variables|Default|GetParent) true true))

(fn ConstructionScript)