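; BP_TankProjectile is the tank enemy's projectile, which holds its place beside the tank before launching and homing on the player.
; BeginPlay picks a BP_TankCharacter by squared-distance check, saves the spawn offset from it and caches the player.
; Until initialized, Tick keeps it at that offset; afterwards it gradually interpolates its direction toward the player.
; DelayedInit waits a given delay before calling InitializeProjectile with the supplied data.
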(event Custom|Delayed%20Init
  (params (Delay :type Float%20%28double-precision%29) (Data :type Projectile%20Data%20Structure))
  (Utilities|FlowControl|Delay Delay)
  (Class|RangedAttackProjectile|InitializeProjectile Data))

(event EventBeginPlay
  (bind _outactors (Actor|GetAllActorsOfClass "/Game/Combat/Enemies/Tank/BP_TankCharacter.BP_TankCharacter_C"))
  (for (_array_element _array_index) _outactors
    (if (< (Class|KismetMathLibrary|VectorDistanceSquared (Transformation|GetActorLocation _array_element) (Transformation|GetActorLocation)) (Variables|Default|GetSavedDist))
      (Variables|Default|SetSavedDist 0.0)
      (Variables|Default|SetSavedIndex _array_index)))
  (bind _output_get (Variables|Default|SetEnemy (Utilities|Array|Get(acopy) _outactors (Variables|Default|GetSavedIndex))))
  (Variables|Default|SetSavedOffset (- (Transformation|GetActorLocation) (Transformation|GetActorLocation _output_get)))
  (bind _returnvalue (Actor|GetActorOfClass "/Game/Player/BP_PlayerCharacter.BP_PlayerCharacter_C"))
  (Variables|Default|Setplayer _returnvalue))

(event Collision|EventActorBeginOverlap
  (params (OtherActor :type Actor%20Object%20Reference)))

(event EventTick
  (params (DeltaSeconds :type Float%20%28single-precision%29))
  (if (Variables|Default|GetIsInitialized)
    (Class|RangedAttackProjectile|SetDirection (Math|Interpolation|RInterpTo (Class|RangedAttackProjectile|GetDirection) (Math|Conversions|RotationFromXVector (- (Transformation|GetActorLocation (Variables|Default|Getplayer)) (Transformation|GetActorLocation))) DeltaSeconds 1.0))
    (else
      (Transformation|SetActorLocation (+ (Transformation|GetActorLocation (Variables|Default|GetEnemy)) (Variables|Default|GetSavedOffset)) false false))))

(fn ConstructionScript
  (|CallParentFunction))