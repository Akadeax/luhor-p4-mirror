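; Tank enemy character with health bar, marked display, and hit flash with splatters.
; Pull and push melee attacks share a growing ground indicator timed to windup.
; During contact, Tick hit-stuns the player within box range and curve-launches them toward or away from the tank.
; Push contact also spawns five projectiles, then fires them staggered at the player.
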(event OnHit(Hittable)
  (params (Data :type Hittable%20Hit%20Data%20Structure))
  (Utilities|FlowControl|Sequence
    (:then_0
      (bind _alpha (Timeline|Timeline PlayFromStart)
        (:Update
          (Rendering|Material|SetScalarParameterValue (Variables|Default|GetDynMat) "FlashingAlpha" _alpha :!class /Script/Engine.MaterialInstanceDynamic))))
    (:then_1
      (Default|SpawnAmbrosiaSplatters (Variables|Default|GetSplatter_Component) 1 2))))

(event OnMeleeAttackCancelled(MeleePullAttack)
  (Utilities|FlowControl|Sequence
    (:then_0
      (Development|SetHiddeninGame (Variables|Default|GetParent) true true)
      (Transformation|SetRelativeScale3D (Variables|Default|GetFillParent) "1.000000,1.000000,1.000000")
      (Transformation|SetRelativeScale3D (Variables|Default|GetParent) "1.000000,1.000000,1.000000"))
    (:then_1
      (bind _scale (Timeline|IndicatorTimeline Stop)
        (:Update
          (Transformation|SetRelativeScale3D (Variables|Default|GetFillParent) (Math|Vector|MakeVector _scale _scale 1.0)))))))

(event OnAttackStateChanged(MeleePullAttack)
  (params (NewState :type EAttackState%20Enum :default "None"))
  (CallFunction|DoAttackIndicator NewState))

(event OnAttackStateChanged(MeleePushAttack)
  (params (NewState :type EAttackState%20Enum :default "None"))
  (CallFunction|DoAttackIndicator NewState)
  (if (Utilities|Enum|Equal(Enum) NewState "Contact")
    (Utilities|FlowControl|Delay (Math|Float|Clamp(Float) (- (.contacttime (Utilities|Array|Get(acopy) (Variables|/Script/LuhorPrototype.MeleeAttackChain|GetAttacks (Variables|/Script/LuhorPrototype.MeleeAttackerComponent|GetMeleeAttackChain (Variables|Default|GetMeleePushAttack))))) 0.1) 0.0 1e+06))
    (Utilities|Array|Clear (Variables|Default|GetTankBulllets))
    (for _index (range 0 4)
      (bind _returnvalue (Game|SpawnActorfromClass "/Game/Combat/Enemies/Tank/BP_TankProjectile.BP_TankProjectile_C" (Math|Transform|MakeTransform (+ (Utilities|Array|Get(acopy) (Variables|Default|GetBulletSpawnLocations) _index) (Transformation|GetActorLocation)) "0, 0, 0" "1.000000,1.000000,1.000000") "Undefined" "MultiplyWithRoot" 0 0))
      (bind _returnvalue_2 (Utilities|Array|Add (Variables|Default|GetTankBulllets) _returnvalue))
      (Development|PrintString (Utilities|String|ToString(Integer) _returnvalue_2)))
    (Utilities|FlowControl|Delay 0.8)
    (for (_array_element _array_index) (Variables|Default|GetTankBulllets)
      (Default|DelayedInit _array_element (* _array_index 0.1) (Utilities|Struct|MakeProjectileData "/Game/Combat/Enemies/Tank/DA_TankRangedAttack.DA_TankRangedAttack" "/Game/Combat/Factions/DA_FactionEnemy.DA_FactionEnemy" self (Math|Conversions|RotationFromXVector (- (Transformation|GetActorLocation (Variables|Default|GetPlayer)) (Transformation|GetActorLocation _array_element))))))))

(event Custom|OnMarkedEnd
  (Class|HeadDisplayWidgetComponent|DeactivateDisplay (Variables|Default|GetMarkedHeadDisplay)))

(event Custom|OnMarked
  (Class|HeadDisplayWidgetComponent|IndefiniteDisplay (Variables|Default|GetMarkedHeadDisplay) "Marked"))

(event Custom|On%20Attack%20Tick
  (params (Reverse :type Integer))
  (bind _self self)
  (bind _player (Variables|Default|GetPlayer))
  (bind _returnvalue (Transformation|GetSquaredDistanceTo _player _self))
  (if (<= _returnvalue (Math|Float|Power (.x (Components|Box|GetScaledBoxExtent (Variables|Default|GetBox))) 2.0))
    (Class|HittableComponent|CustomHitStun (Variables|/Game/Player/BP_PlayerCharacter.BP_PlayerCharacter_C|GetHittable _player) 0.2)
    (if (or (> _returnvalue 1e+04) (== Reverse -1))
      (Class|LuhorMovementComponent|DoCurvedLaunch (Variables|/Script/LuhorPrototype.LuhorCharacter|GetLuhorCharacterMovement _player) (* (- (Transformation|GetWorldLocation (Variables|Default|GetBox)) (Transformation|GetWorldLocation (Variables|/Script/Engine.Actor|GetRootComponent _player))) Reverse) (Utilities|Struct|MakeCurvedLaunchData 0.1 (Math|Float|SelectFloat 15.0 2e+02 (== Reverse 1)) "/Game/Combat/Enemies/Tank/C_InstantPulse.C_InstantPulse")))))

(event Custom|DoAttackIndicator
  (params (NewParam :type EAttackState%20Enum :default "None"))
  (if (Utilities|Enum|Equal(Enum) NewParam "Windup")
    (Components|Timeline|SetPlayRate (Variables|Default|GetIndicatorTimeline) (/ 1.0 (.winduptime (Utilities|Array|Get(acopy) (Variables|/Script/LuhorPrototype.MeleeAttackChain|GetAttacks (Variables|/Script/LuhorPrototype.MeleeAttackerComponent|GetMeleeAttackChain (Variables|Default|GetMeleePullAttack)))))))
    (Development|SetHiddeninGame (Variables|Default|GetParent) false true)
    (bind _scale (Timeline|IndicatorTimeline PlayFromStart)
      (:Update
        (Transformation|SetRelativeScale3D (Variables|Default|GetFillParent) (Math|Vector|MakeVector _scale _scale 1.0))))
    (elif (not (Utilities|Enum|Equal(Enum) NewParam "Contact"))
      (if (Utilities|Enum|Equal(Enum) NewParam "Recovery")
        (Development|SetHiddeninGame (Variables|Default|GetParent) true true)
        (Transformation|SetRelativeScale3D (Variables|Default|GetFillParent) "1.000000,1.000000,1.000000")
        (Transformation|SetRelativeScale3D (Variables|Default|GetParent) "1.000000,1.000000,1.000000")))))

(event EventBeginPlay
  (bind _headdisplaywidget (Variables|Default|GetHeadDisplayWidget))
  (bind _markedheaddisplay (Variables|Default|GetMarkedHeadDisplay))
  (bind _hittable (Variables|Default|GetHittable))
  (bind _returnvalue (Rendering|Material|CreateDynamicMaterialInstance (Variables|Character|GetMesh) 0 (Rendering|Material|GetMaterial (Variables|Character|GetMesh) 0) "None" :!class /Script/Engine.PrimitiveComponent))
  (bind _output_get (Variables|Default|SetDynMat _returnvalue))
  (Rendering|Material|SetMaterial (Variables|Character|GetMesh) 0 _output_get)
  (bind _returnvalue_2 (Game|ConstructObjectfromClass "/Game/Combat/WBP_EntityHealthBar.WBP_EntityHealthBar_C" (Variables|Default|GetHealth) (Variables|Default|GetStagger) (Variables|Default|GetHittable)))
  (UserInterface|SetWidget (Variables|Default|GetHealthBar) _returnvalue_2)
  (bind _returnvalue_3 (Game|ConstructObjectfromClass "/Game/Combat/WBP_HeadDisplayWidget.WBP_HeadDisplayWidget_C" _headdisplaywidget))
  (UserInterface|SetWidget _headdisplaywidget _returnvalue_3)
  (EventDispatchers|BindEventtoOnMarked _hittable (delegate Custom|OnMarked))
  (EventDispatchers|BindEventtoOnMarkConsumed _hittable (delegate Custom|OnMarkedEnd))
  (bind _returnvalue_4 (Game|ConstructObjectfromClass "/Game/Combat/WBP_HeadDisplayWidget.WBP_HeadDisplayWidget_C" _markedheaddisplay))
  (UserInterface|SetWidget _markedheaddisplay _returnvalue_4)
  (Development|SetHiddeninGame (Variables|Default|GetParent) true true)
  (bind _outactors (Actor|GetAllActorsOfClass "/Game/Player/BP_PlayerCharacter.BP_PlayerCharacter_C"))
  (Variables|Default|SetPlayer (Utilities|Array|Get(acopy) _outactors))
  (Transformation|SetRelativeTransform (Variables|Default|GetBox1) (Transformation|GetRelativeTransform (Variables|Default|GetBox)) false true))

(event EventTick
  (params (DeltaSeconds :type Float%20%28single-precision%29))
  (Utilities|FlowControl|Sequence
    (:then_0
      (if (Utilities|Enum|Equal(Enum) (Variables|/Script/LuhorPrototype.BaseAttackerComponent|GetCurrentAttackState (Variables|Default|GetMeleePullAttack)) "Contact")
        (CallFunction|OnAttackTick 1)))
    (:then_1
      (if (Utilities|Enum|Equal(Enum) (Variables|/Script/LuhorPrototype.BaseAttackerComponent|GetCurrentAttackState (Variables|Default|GetMeleePushAttack)) "Contact")
        (CallFunction|OnAttackTick -1)))))

(fn ConstructionScript)