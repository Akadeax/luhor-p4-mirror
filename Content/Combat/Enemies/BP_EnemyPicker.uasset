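; Enemy combat director that picks random enemies to attack or taunt based on their distance to the player.
; Tick drives both pickers, throttled by Delays to about one and five seconds.
; Nearby unstaggered fast-melee enemies may get TryAttack; farther enemies may halt for a taunt montage, then resume walking.
; The taunt picker clears the melee list instead of its own, so its candidates accumulate.
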(event Custom|Melee%20Attack%20Picker
  (bind _currentlyviable (Variables|Default|GetCurrentlyViable))
  (Utilities|FlowControl|Delay 1.0)
  (Utilities|Array|Clear (Variables|Default|GetCurrentlyViable))
  (bind _outactors (Actor|GetAllActorsOfClass "/Game/Combat/Enemies/FastMelee/BP_FastMeleeCharacter.BP_FastMeleeCharacter_C"))
  (for _array_element _outactors
    (if (and (not (Class|StaggerComponent|GetStaggered (Variables|/Game/Combat/Enemies/FastMelee/BP_FastMeleeCharacter.BP_FastMeleeCharacter_C|GetStagger _array_element))) (< (Transformation|GetDistanceTo (Variables|Default|GetPlayer) _array_element) 3.5e+02))
      (Utilities|Array|Add (Variables|Default|GetCurrentlyViable) _array_element)))
  (if (> (Utilities|Array|Length _currentlyviable) 0)
    (bind _output_get (Variables|Default|SetTempMeleeEnemy (.OutItem (Utilities|Array|Random _currentlyviable))))
    (Utilities|IsValid _output_get
      (:Is%20Valid
        (Class|BaseAttackerComponent|TryAttack (Variables|/Game/Combat/Enemies/FastMelee/BP_FastMeleeCharacter.BP_FastMeleeCharacter_C|GetMeleeAttacker _output_get))))))

(event Custom|tauntPicker
  (bind _currentlyviable_0 (Variables|Default|GetCurrentlyViable_0))
  (Utilities|FlowControl|Delay 5.0)
  (Utilities|Array|Clear (Variables|Default|GetCurrentlyViable))
  (bind _outactors (Actor|GetAllActorsOfClass "/Script/LuhorPrototype.LuhorEnemyCharacter"))
  (for _array_element _outactors
    (if (> (Transformation|GetDistanceTo (Variables|Default|GetPlayer) _array_element) 351.0)
      (Utilities|Array|Add _currentlyviable_0 _array_element)))
  (if (> (Utilities|Array|Length _currentlyviable_0) 0)
    (bind _output_get (Variables|Default|SetTempEnemy (.OutItem (Utilities|Array|Random _currentlyviable_0))))
    (Utilities|IsValid _output_get
      (:Is%20Valid
        (Variables|/Script/Engine.CharacterMovementComponent|SetMaxWalkSpeed (Variables|/Script/LuhorPrototype.LuhorCharacter|GetLuhorCharacterMovement _output_get) 0.0)
        (Development|PrintString "BeezleBorp")
        (Animation|Montage|PlayMontage (Variables|/Script/Engine.Character|GetMesh _output_get) "/Game/Combat/Enemies/FastMelee/Anim/AM_EnemyTaunt.AM_EnemyTaunt"
          (:OnCompleted
            (Variables|/Script/Engine.CharacterMovementComponent|SetMaxWalkSpeed (Variables|/Script/LuhorPrototype.LuhorCharacter|GetLuhorCharacterMovement _output_get) 2e+02)))))))

(event EventTick
  (params (DeltaSeconds :type Float%20%28single-precision%29))
  (Utilities|FlowControl|Sequence
    (:then_0
      (CallFunction|MeleeAttackPicker))
    (:then_1
      (CallFunction|TauntPicker))))

(event EventBeginPlay
  (bind _returnvalue (Actor|GetActorOfClass "/Game/Player/BP_PlayerCharacter.BP_PlayerCharacter_C"))
  (Variables|Default|SetPlayer _returnvalue))

(fn ConstructionScript)