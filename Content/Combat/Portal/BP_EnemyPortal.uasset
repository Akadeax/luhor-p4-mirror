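; Enemy portal that spawns enemies at randomly offset points nearby and shows its health on a bar.
; It loses health steadily and with each spawn, by a per-class cost, and a curve maps remaining health to the next spawn interval.
; Spawn selection rolls against a weighted map, then upgrades melee or ranged picks to stronger variants based on capped rooms completed, defaulting any other class to fast melee.
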(event Custom|SpawnEnemy
  (bind _class (CallFunction|GetWeightedEnemyClass))
  (Game|SpawnActorfromClass _class (Math|Transform|MakeTransform (+ (Variables|Default|GetSpawnLocations) (* (Math|Random|RandomUnitVector) (Math|Random|RandomFloatinRange 0.0 (Variables|Default|GetOfsetSpawnDist))) (Transformation|GetActorLocation)) "0, 0, 0" "1.000000,1.000000,1.000000") "AdjustIfPossibleButAlwaysSpawn" "MultiplyWithRoot" 0 0)
  (Class|HealthComponent|Damage (Variables|Default|GetHealth) (.Value (Utilities|Map|Find (Variables|Default|GetEnemyDamageMap) _class))))

(event EventBeginPlay
  (CallFunction|SpawnEnemy)
  (bind _returnvalue (Game|ConstructObjectfromClass "/Game/Combat/WBP_EntityHealthBar.WBP_EntityHealthBar_C" (Variables|Default|GetHealth) 0))
  (UserInterface|SetWidget (Variables|Default|GetHealthBar) _returnvalue)
  (Variables|Default|SetCurrent%20Time%20Between%20Spawns (Variables|Default|GetMax%20Time%20Between%20Spawns)))

(event EventTick
  (params (DeltaSeconds :type Float%20%28single-precision%29))
  (bind _health (Variables|Default|GetHealth))
  (Utilities|FlowControl|Sequence
    (:then_0
      (if (<= (Variables|Default|GetCurrent%20Time%20Between%20Spawns) 0.0)
        (CallFunction|SpawnEnemy)
        (Variables|Default|SetCurrent%20Time%20Between%20Spawns (* (Variables|Default|GetMax%20Time%20Between%20Spawns) (Math|Curves|GetFloatValue (Variables|Default|GetHealthToTimeGraph) (/ (Class|HealthComponent|GetCurrentHealth _health) (Class|HealthComponent|GetMaxHealth _health)))))
        (else
          (Variables|Default|SetCurrent%20Time%20Between%20Spawns (- (Variables|Default|GetCurrent%20Time%20Between%20Spawns) DeltaSeconds)))))
    (:then_1
      (Class|HealthComponent|Damage (Variables|Default|GetHealth) (* DeltaSeconds (Variables|Default|GetDamagePerSec))))))

(fn ConstructionScript)

(fn GetWeightedEnemyClass
  (LocalVariables|SetRandomWeight (Math|Random|RandomFloatinRange 0.0 1.0))
  (bind (_keypin _valuepin) (Utilities|Map|ForEachLoop(Map) (Variables|Default|GetEnemyProbabilities))
    (:then
      (if (<= (LocalVariables|GetRandomWeight) _valuepin)
        (LocalVariables|SetRandomWeight (Math|Random|RandomFloatinRange 0.0 1e+02))
        (bind _returnvalue (Class|LevelGameInstanceSubsystem|GetRoomsCompleted (Subsystems|GetLevelGameInstanceSubsystem)))
        (if (== _keypin "/Game/Combat/Enemies/FastMelee/BP_FastMeleeCharacter.BP_FastMeleeCharacter_C")
          (if (> (- 100 (* (Math|Integer|Clamp(Integer) _returnvalue 0 5) 20)) (LocalVariables|GetRandomWeight))
            _
            (elif (>= (+ (* (Math|Integer|Clamp(Integer) _returnvalue 0 5) 15) (- 100 (* (Math|Integer|Clamp(Integer) _returnvalue 0 5) 20))) (LocalVariables|GetRandomWeight))
              (return "/Game/Combat/Enemies/FastMelee/BP_FasterMeleeCharacter.BP_FasterMeleeCharacter_C")
              (elif (>= (+ (* (Math|Integer|Clamp(Integer) _returnvalue 0 5) 5) (* (Math|Integer|Clamp(Integer) _returnvalue 0 5) 15) (- 100 (* (Math|Integer|Clamp(Integer) _returnvalue 0 5) 20))) (LocalVariables|GetRandomWeight))
                (return "/Game/Combat/Enemies/FastMelee/BP_FastestMeleeCharacter.BP_FastestMeleeCharacter_C")
                (else
                  _))))
          (elif (== _keypin "/Game/Combat/Enemies/Ranged/BP_RangedCharacter.BP_RangedCharacter_C")
            (if (> (- 100 (* (Math|Integer|Clamp(Integer) _returnvalue 0 5) 15)) (LocalVariables|GetRandomWeight))
              (return "/Game/Combat/Enemies/Ranged/BP_RangedCharacter.BP_RangedCharacter_C")
              (else
                (return "/Game/Combat/Enemies/Ranged/BP_RangedCharacterCooler.BP_RangedCharacterCooler_C")))
            (else
              _)))
        (return "/Game/Combat/Enemies/FastMelee/BP_FastMeleeCharacter.BP_FastMeleeCharacter_C")
        (else
          (LocalVariables|SetRandomWeight (- (LocalVariables|GetRandomWeight) _valuepin)))))
    (:CompletedPin
      (return "/Game/Combat/Enemies/FastMelee/BP_FastMeleeCharacter.BP_FastMeleeCharacter_C"))))