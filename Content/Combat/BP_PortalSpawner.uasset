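; Combat encounter spawner that spawns an enemy group on BeginPlay when active, then opens enemy portals.
; Enemies appear around random spawn locations, with class rolls scaled by completed rooms and a WeaknessType assigned to each.
; It also reserves two locations and marks them with spore Niagara effects.
; The first OnEnemyDied call spawns BP_EnemyPortal at both marks and removes the effects.
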(event Custom|OnEnemyDied
  (Utilities|FlowControl|DoOnce false
    (:Completed
      (for _array_element (Variables|Default|GetPickedSpawns)
        (Game|SpawnActorfromClass "/Game/Combat/Portal/BP_EnemyPortal.BP_EnemyPortal_C" (Math|Transform|MakeTransform _array_element "0, 0, 0" "1.000000,1.000000,1.000000") "AdjustIfPossibleButAlwaysSpawn" "MultiplyWithRoot" 0 0))
      (for _array_element_2 (Variables|Default|Getniagara)
        (Components|DestroyComponent _array_element_2)))))

(event Custom|SpawnGroup1
  (bind _groupsleft (Variables|Default|GetGroupsLeft))
  (bind _enemygroup1 (Variables|Default|GetEnemyGroup1))
  (Utilities|Array|Clear _enemygroup1)
  (if (> _groupsleft 0)
    (Math|Integer|DecrementInt _groupsleft
      (:%20%20
        (for _index (range 1 (Math|Random|RandomIntegerinRange (Variables|Default|GetMinEnemiesPerGroup) (Variables|Default|GetMaxEnemiesPerGroup)))
          (bind _class (CallFunction|GetWeightedEnemyClass))
          (bind _returnvalue (Game|SpawnActorfromClass _class (Math|Transform|MakeTransform (+ (.OutItem (Utilities|Array|Random (Variables|Default|GetSpawnLocations))) (* (Math|Random|RandomUnitVector) (Math|Random|RandomFloatinRange 0.0 (Variables|Default|GetOfsetSpawnDist))) (Transformation|GetActorLocation)) "0, 0, 0" "1.000000,1.000000,1.000000") "AdjustIfPossibleButAlwaysSpawn" "MultiplyWithRoot" 0 0))
          (bind _weakness (CallFunction|GetWeightedResistance))
          (Variables|/Script/LuhorPrototype.HittableComponent|SetWeaknessType (Actor|GetComponentbyClass _returnvalue "/Script/LuhorPrototype.HittableComponent") _weakness)
          (Utilities|Array|Add _enemygroup1 _returnvalue)
          (EventDispatchers|BindEventtoOnDeath (Actor|GetComponentbyClass _returnvalue "/Script/LuhorPrototype.HealthComponent") (EventDispatchers|CreateEvent :!event Custom|OnEnemyDied)))))))

(event EventBeginPlay
  (bind _spawnlocations (Variables|Default|GetSpawnLocations))
  (if (Variables|Default|GetIsActive)
    (if (!= (Utilities|Array|Length (Variables|Default|GetSpawnLocations)) 0)
      (Variables|Default|SetGroupsLeft (Variables|Default|GetGroupsPerWave))
      (CallFunction|SpawnGroup1)
      (Utilities|FlowControl|DoOnce false
        (:Completed
          (for _index (range 0 1)
            (bind _output_get (Variables|Default|Settemp (.OutItem (Utilities|Array|Random _spawnlocations))))
            (Utilities|Array|Add (Variables|Default|GetPickedSpawns) (+ _output_get (Transformation|GetActorLocation)))
            (Utilities|Array|RemoveItem _spawnlocations _output_get)
            (bind _returnvalue (Niagara|SpawnSystematLocation "/Game/VFX/Spores/FXS_Spores.FXS_Spores" (+ _output_get (Transformation|GetActorLocation)) "0, 0, 0" "0.250000,0.250000,1.000000"))
            (Utilities|Array|Add (Variables|Default|Getniagara) _returnvalue))))
      (else
        (Utilities|Debugging|RaiseScriptError "EnemySpawner doesnt have any spawn locations")))))

(fn ConstructionScript)

(fn GetWeightedEnemyClass
  (bind _returnvalue (Math|Random|RandomFloatinRange 0.0 1e+02))
  (bind _returnvalue_2 (Class|LevelGameInstanceSubsystem|GetRoomsCompleted (Subsystems|GetLevelGameInstanceSubsystem)))
  (if (> _returnvalue (- 100 (+ (* (Math|Integer|Clamp(Integer) _returnvalue_2 0 5) 2) 5)))
    (return "/Game/Combat/Enemies/Tank/BP_TankCharacter.BP_TankCharacter_C")
    (elif (> _returnvalue (- (- 100 (+ (* (Math|Integer|Clamp(Integer) _returnvalue_2 0 5) 2) 5)) (+ (* (Math|Integer|Clamp(Integer) _returnvalue_2 0 5) 4) 15)))
      (return "/Game/Combat/Enemies/Ranged/BP_RangedCharacter.BP_RangedCharacter_C")
      (else
        (return "/Game/Combat/Enemies/FastMelee/BP_FastMeleeCharacter.BP_FastMeleeCharacter_C")))))

(fn ShouldGroupRespawn
  (params (Group :type Array%20of%20Luhor%20Enemy%20Character%20Object%20References))
  (for _array_element Group
    (if (Utilities|IsValid _array_element)
      (if (> (Class|HealthComponent|GetCurrentHealth (Actor|GetComponentbyClass _array_element "/Script/LuhorPrototype.HealthComponent")) 0.0)
        (return false))))
  (return true))

(fn GetWeightedResistance
  (bind _returnvalue (Class|LevelGameInstanceSubsystem|GetRoomsCompleted (Subsystems|GetLevelGameInstanceSubsystem)))
  (if (> (* (Math|Integer|Clamp(Integer) _returnvalue 0 5) 10) (Math|Random|RandomFloatinRange 0.0 1e+02))
    (return "None")
    (else
      (return "None"))))