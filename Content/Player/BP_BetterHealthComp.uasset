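; BP_BetterHealthComp is a player health component that counts health in pips, starting full.
; It binds to the player's Hittable and both melee attackers.
; Landed melee hits build progress toward regaining a pip while below the maximum.
; Each hit taken halves that progress and removes one pip regardless of damage, and a hit at zero pips quits the game.
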(event Custom|OnHit
  (params (Data :type Hittable%20Hit%20Data%20Structure))
  (CallFunction|ResetProgress?)
  (if (> (Variables|Default|GetCurrentPips) 0)
    (Math|Integer|DecrementInt (Variables|Default|GetCurrentPips))
    (else
      (Game|QuitGame 0 "Quit" true))))

(event Custom|OnEnemyhit
  (params (Data :type Hittable%20Hit%20Data%20Structure) (WasLethal :type Boolean) (Hittable :type Hittable%20Component%20Object%20Reference))
  (if (< (Variables|Default|GetCurrentPips) (Variables|Default|GetMaxPips))
    (Variables|Default|SetCurrentProgressToNext (+ (Variables|Default|GetCurrentProgressToNext) (/ 1.0 (Math|Conversions|ToFloat(Integer) (Variables|Default|GetHitsToGetOnePip)))))
    (if (>= (Variables|Default|GetCurrentProgressToNext) 0.99)
      (Variables|Default|SetCurrentProgressToNext 0.0)
      (Math|Integer|IncrementInt (Variables|Default|GetCurrentPips)))
    (else
      (Variables|Default|SetCurrentProgressToNext 0.0))))

(event EventBeginPlay
  (bind _asbp_player_character (Utilities|Casting|CastToBP_PlayerCharacter (Components|GetOwner)))
  (Variables|Default|SetPlayer _asbp_player_character)
  (Variables|Default|SetCurrentPips (Variables|Default|GetMaxPips))
  (EventDispatchers|BindEventtoOnHit (Variables|/Game/Player/BP_PlayerCharacter.BP_PlayerCharacter_C|GetHittable (Variables|Default|GetPlayer)) (delegate Custom|OnHit))
  (EventDispatchers|BindEventtoOnMeleeAttackHit (Variables|/Game/Player/BP_PlayerCharacter.BP_PlayerCharacter_C|GetPrimaryMeleeAttacker (Variables|Default|GetPlayer)) (delegate Custom|OnEnemyhit))
  (EventDispatchers|BindEventtoOnMeleeAttackHit (Variables|/Game/Player/BP_PlayerCharacter.BP_PlayerCharacter_C|GetSecondaryMeleeAttacker (Variables|Default|GetPlayer)) (delegate Custom|OnEnemyhit)))

(fn ResetProgress?
  (Variables|Default|SetCurrentProgressToNext (/ (Variables|Default|GetCurrentProgressToNext) 2.0)))