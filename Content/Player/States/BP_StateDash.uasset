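; Player dash state that gates dashing behind a cooldown and makes the character briefly invulnerable on entry through its Hittable.
; Tick counts the cooldown down, and CanEnterState requires it to have expired before deferring to the parent check.
; A successful check starts the cooldown as a side effect, tripled when the owner's UpgradesComponent holds a GhostUpgrade subclass.
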(event EventTick
  (params (DeltaSeconds :type Float%20%28single-precision%29))
  (if (> (Variables|Default|GetAttackCooldownLeft) 0.0)
    (Variables|Default|SetAttackCooldownLeft (- (Variables|Default|GetAttackCooldownLeft) DeltaSeconds))))

(event EventOnEnterState
  (|CallParentFunction)
  (Class|HittableComponent|MakeInvulnerable (Variables|/Game/Player/BP_PlayerCharacter.BP_PlayerCharacter_C|GetHittable (CallFunction|GetCharacter)) 0.3 "SetTimeIfLonger"))

(fn CanEnterState
  (bind _attackcooldown (Variables|Default|GetAttackCooldown))
  (if (<= (Variables|Default|GetAttackCooldownLeft) 0.0)
    (bind _returnvalue (|CallParentFunction))
    (if _returnvalue
      (if true
        (bind _return (CallFunction|HasGhostUpgrade))
        (Variables|Default|SetAttackCooldownLeft (Math|Float|SelectFloat (* _attackcooldown 3.0) _attackcooldown _return))
        (return _returnvalue))
      (else
        (return _returnvalue)))
    (else
      (return false))))

(fn GetDependencies
  (return 0))

(fn HasGhostUpgrade
  (for _array_element (Class|UpgradesComponent|GetUpgrades (Actor|GetComponentbyClass (Components|GetOwner) "/Script/LuhorPrototype.UpgradesComponent"))
    (if (Utilities|ClassIsChildOf _array_element "/Script/LuhorPrototype.GhostUpgrade")
      (return true)))
  (return false))