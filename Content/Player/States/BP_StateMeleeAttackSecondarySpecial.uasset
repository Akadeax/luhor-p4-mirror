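; Player state machine state for the secondary special melee attack.
; It binds to the character's dash input event on enter and unbinds it on exit.
; Secondary attack input sets control rotation from move input with an angular offset, then requests the Dash state.
; Primary attack input does nothing, and the attack call is disconnected, so this graph never triggers an attack itself.
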(event Custom|OnInputPrimaryAttackTriggered)

(event Custom|OnInputSecondaryAttackTriggered
  (bind _currentmoveinput (Variables|Default|GetCurrentMoveInput))
  (Class|LuhorCharacter|SetControlRotationfromInputDir (CallFunction|GetCharacter) (Math|Vector|MakeVector (.x _currentmoveinput) (.y _currentmoveinput) 0.0) 9e+01)
  (Class|StateMachineComponent|TryChangeState (Class|SMStateComponent|GetStateMachine) "Dash"))

(event EventOnEnterState
  (|CallParentFunction)
  (EventDispatchers|BindEventtoOnInputDashTriggered (CallFunction|GetCharacter) (EventDispatchers|CreateEvent :!event Custom|OnInputSecondaryAttackTriggered)))

(event EventOnExitState
  (|CallParentFunction)
  (EventDispatchers|UnbindEventfromOnInputDashTriggered (CallFunction|GetCharacter) (EventDispatchers|CreateEvent :!event Custom|OnInputSecondaryAttackTriggered)))

(fn GetDependencies
  (return 0))