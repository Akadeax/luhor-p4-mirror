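; Player state for the secondary melee attack, gated by a cooldown that counts down on Tick.
; While active it binds secondary attack, primary attack and dash inputs to attack again or switch to SecondarySpecialAttack or Dash.
; Both transitions first set control rotation from the movement input.
; CanEnterState also starts the cooldown when it passes, so the check itself has a side effect.
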(event Custom|OnInputSecondaryAttack
  (Class|MeleeAttackerComponent|TryAttack (Variables|Default|GetAttacker)))

(event Custom|OnDash
  (bind _currentmoveinput (Variables|Default|GetCurrentMoveInput))
  (Class|LuhorCharacter|SetControlRotationfromInputDir (CallFunction|GetCharacter) (Math|Vector|MakeVector (.x _currentmoveinput) (.y _currentmoveinput) 0.0) 9e+01)
  (Class|StateMachineComponent|TryChangeState (Class|SMStateComponent|GetStateMachine) "Dash"))

(event Custom|OnMeleeattackSecondarySpecial
  (bind _currentmoveinput (Variables|Default|GetCurrentMoveInput))
  (Class|LuhorCharacter|SetControlRotationfromInputDir (CallFunction|GetCharacter) (Math|Vector|MakeVector (.x _currentmoveinput) (.y _currentmoveinput) 0.0) 9e+01)
  (Class|StateMachineComponent|TryChangeState (Class|SMStateComponent|GetStateMachine) "SecondarySpecialAttack"))

(event EventTick
  (params (DeltaSeconds :type Float%20%28single-precision%29))
  (if (> (Variables|Default|GetAttackCooldownLeft) 0.0)
    (Variables|Default|SetAttackCooldownLeft (- (Variables|Default|GetAttackCooldownLeft) DeltaSeconds))))

(event EventOnEnterState
  (|CallParentFunction)
  (EventDispatchers|BindEventtoOnInputSecondaryAttackTriggered (CallFunction|GetCharacter) (EventDispatchers|CreateEvent :!event Custom|OnInputSecondaryAttack))
  (EventDispatchers|BindEventtoOnInputDashTriggered (CallFunction|GetCharacter) (EventDispatchers|CreateEvent :!event Custom|OnDash))
  (EventDispatchers|BindEventtoOnInputPrimaryAttackTriggered (CallFunction|GetCharacter) (EventDispatchers|CreateEvent :!event Custom|OnMeleeattackSecondarySpecial)))

(event EventOnExitState
  (|CallParentFunction)
  (EventDispatchers|UnbindEventfromOnInputSecondaryAttackTriggered (CallFunction|GetCharacter) (EventDispatchers|CreateEvent :!event Custom|OnInputSecondaryAttack))
  (EventDispatchers|UnbindEventfromOnInputDashTriggered (CallFunction|GetCharacter) (EventDispatchers|CreateEvent :!event Custom|OnDash))
  (EventDispatchers|UnbindEventfromOnInputPrimaryAttackTriggered (CallFunction|GetCharacter) (EventDispatchers|CreateEvent :!event Custom|OnMeleeattackSecondarySpecial)))

(fn CanEnterState
  (if (<= (Variables|Default|GetAttackCooldownLeft) 0.0)
    (bind _returnvalue (|CallParentFunction))
    (if _returnvalue
      (if true
        (Variables|Default|SetAttackCooldownLeft (Variables|Default|GetAttackCooldown))
        (return _returnvalue))
      (else
        (return _returnvalue)))
    (else
      (return false))))